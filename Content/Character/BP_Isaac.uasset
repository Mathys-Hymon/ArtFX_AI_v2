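; BP_Isaac is a player character Blueprint that extends a parent's shooting and handles its own damage and death.
; Shoot passes a camera-origin, control-rotation trace segment to the parent, then damages blocking-hit actors that pass an interface check.
; It also writes the hit actor into the blackboard of the BP_Ally found at BeginPlay, setting the ally's target.
; Incoming damage reduces Health, and reaching zero opens the L_Dust3 level.
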(event EventBeginPlay
  (|CallParentFunction)
  (bind _returnvalue (Actor|GetActorOfClass "/Game/Character/BP_Ally.BP_Ally_C"))
  (Variables|Default|SetAllyRef _returnvalue))

(event Collision|EventActorBeginOverlap
  (params (OtherActor :type Actor%20Object%20Reference))
  (|CallParentFunction OtherActor) ; This node is disabled and will not be called.\nDrag off pins to build functionality.
)

(event EventTick
  (params (DeltaSeconds :type Float%20%28single-precision%29))
  (|CallParentFunction DeltaSeconds) ; This node is disabled and will not be called.\nDrag off pins to build functionality.
)

(event Game|Damage|EventAnyDamage
  (params (Damage :type Float%20%28single-precision%29) (DamageType :type Damage%20Type%20Object%20Reference) (InstigatedBy :type Controller%20Object%20Reference) (DamageCauser :type Actor%20Object%20Reference))
  ;[1 0.01175 0] Die
  (bind _output_get (Variables|Default|SetHealth (- (Variables|Default|GetHealth) Damage)))
  (if (<= _output_get 0.0)
    (Game|OpenLevel(byObjectReference) "/Game/Maps/L_Dust3.L_Dust3")))

(event EventShoot
  (params (Start :type Vector :default "0, 0, 0") (End :type Vector :default "0, 0, 0"))
  (bind _returnvalue (Game|GetPlayerCameraManager 0))
  (bind _shoothit (Variables|Default|GetShootHit))
  (bind _returnvalue_2 (Transformation|GetActorLocation _returnvalue))
  (bind (_bblockinghit _binitialoverlap _time _distance _location _impactpoint _normal _impactnormal _physmat _hitactor) (Collision|BreakHitResult _shoothit))
  ;[0 0 0] Shoot
  (|CallParentFunction _returnvalue_2 (+ _returnvalue_2 (* (Math|Vector|GetForwardVector (Pawn|GetControlRotation :!class /Script/Engine.Pawn)) (Variables|Default|GetShootRange))))
  (if _bblockinghit
    (if (Utilities|DoesObjectImplementInterface _hitactor 0)
      (Game|Damage|ApplyDamage _hitactor 1.0 0 0)
      (Utilities|IsValid (Variables|Default|GetAllyRef)
        (:Is%20Valid
          (AI|Components|Blackboard|SetValueasObject (AI|GetBlackboard (Variables|Default|GetAllyRef)) (Variables|Default|GetTargetRefKey) _hitactor))))))

(fn ConstructionScript
  (|CallParentFunction))