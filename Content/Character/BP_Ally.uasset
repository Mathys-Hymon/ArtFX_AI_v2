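; BP_Ally is an ally character Blueprint that reacts to damage by updating its AI target.
; On BeginPlay it caches player character 0 as a BP_Isaac reference.
; Any damage writes the instigating controller, rather than its pawn, to the blackboard's target key through SetTargetRef, then prints a debug message.
; Tick and overlap events are disabled, and the construction script only calls its parent.
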(event EventBeginPlay
  (|CallParentFunction)
  (bind _asbp_isaac (Utilities|Casting|CastToBP_Isaac (Game|GetPlayerCharacter 0)))
  (Variables|Default|SetPlayerRef _asbp_isaac))

(event Collision|EventActorBeginOverlap
  (params (OtherActor :type Actor%20Object%20Reference))
  (|CallParentFunction OtherActor) ; This node is disabled and will not be called.\nDrag off pins to build functionality.
)

(event EventTick
  (params (DeltaSeconds :type Float%20%28single-precision%29))
  (|CallParentFunction DeltaSeconds) ; This node is disabled and will not be called.\nDrag off pins to build functionality.
)

(event Game|Damage|EventAnyDamage
  (params (Damage :type Float%20%28single-precision%29) (DamageType :type Damage%20Type%20Object%20Reference) (InstigatedBy :type Controller%20Object%20Reference) (DamageCauser :type Actor%20Object%20Reference))
  (CallFunction|SetTargetRef InstigatedBy)
  (Development|PrintString "Ouich"))

(fn ConstructionScript
  (|CallParentFunction))

(fn SetTargetRef
  (params (ObjectValue :type Object%20Object%20Reference))
  (AI|Components|Blackboard|SetValueasObject (AI|GetBlackboard 0) (Variables|Default|GetTargetRefKey) ObjectValue))