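; BP_BaseCharacter is a base character with health, a hitscan shoot event and AI-audible noise.
; Shoot line-traces for Pawn objects with debug drawing, stores the hit without applying damage, and makes a "Hearing" noise at the character's location.
; AnyDamage subtracts from Health and opens the L_Dust3 level once it reaches zero or below.
; A Q debug key emits the same noise with itself as instigator.
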(event Custom|Shoot
  (params (Start :type Vector) (End :type Vector))
  (bind _outhit (Collision|LineTraceForObjects Start End (Utilities|Array|MakeArray "ObjectTypeQuery3") false 0 "ForDuration" true "(R=1.000000,G=0.000000,B=0.000000,A=1.000000)" "(R=0.000000,G=1.000000,B=0.000000,A=1.000000)" 1.0))
  (Variables|Default|SetShootHit _outhit)
  (Class|Actor|MakeNoise 1.0 0 (Transformation|GetActorLocation) 0.0 "Hearing"))

(event EventBeginPlay)

(event Collision|EventActorBeginOverlap
  (params (OtherActor :type Actor%20Object%20Reference)))

(event EventTick
  (params (DeltaSeconds :type Float%20%28single-precision%29)))

(event Game|Damage|EventAnyDamage
  (params (Damage :type Float%20%28single-precision%29) (DamageType :type Damage%20Type%20Object%20Reference) (InstigatedBy :type Controller%20Object%20Reference) (DamageCauser :type Actor%20Object%20Reference))
  (bind _output_get (Variables|Default|SetHealth (- (Variables|Default|GetHealth) Damage)))
  (if (<= _output_get 0.0)
    (Game|OpenLevel(byObjectReference) "/Game/Maps/L_Dust3.L_Dust3")))

(event Input|KeyboardEvents|DebugKeyQ
  (params (Key :type Key%20Structure :default "None") (ActionValue :type Input%20Action%20Value%20Structure))
  (:Pressed
    (Class|Actor|MakeNoise 1.0 self (Transformation|GetActorLocation) 0.0 "Hearing")))

(fn ConstructionScript)